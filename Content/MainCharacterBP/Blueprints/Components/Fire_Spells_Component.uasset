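; Fire spell component for the main character that handles casting and launching the Fireball attack.
; FireballAttack, gated by a DoOnce, spawns a short-lived casting effect at the character's SpellDirection and plays the attack montage.
; A separate FireballSpellCasting function spawns the Fireball actor at that same transform.
; EndFireballAttack resets the DoOnce so the attack can fire again.
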(event `self.ReceiveBeginPlay`
  (set `self.As Main Character BP` (cast `/Game/MainCharacterBP/Blueprints/MainCharacterBP` (`GameplayStatics.GetPlayerCharacter` 0) :!pure true)))

(event `Fireball Attack`
  (`/Engine/EditorBlueprintResources/StandardMacros.DoOnce` false :!label _label
    (:`Completed`
      ;[1 1 1] Effect on casting
      (bind _returnvalue (`|SpawnActorFromClass` "/Game/MainCharacterBP/Blueprints/Spells/FireballCasting.FireballCasting_C" (`SceneComponent.K2_GetComponentToWorld` (`/Game/MainCharacterBP/Blueprints/MainCharacterBP.SpellDirection` (`self.As Main Character BP`))) "Undefined" "OverrideRootScale" null null))
      ;[1 1 1] Casting animation
      (`Character.PlayAnimMontage` (`self.As Main Character BP`) "/Game/BattleWizardPolyart/Animations/Attack04Anim_Montage.Attack04Anim_Montage" 1.0 "None")
      (`KismetSystemLibrary.Delay` 0.3)
      (`Actor.K2_DestroyActor` _returnvalue))))

(event `End Fireball Attack`
  (goto _label :!via `Reset`))

(fn `Fireball Spell Casting`
  (`|SpawnActorFromClass` "/Game/MainCharacterBP/Blueprints/Spells/Fireball.Fireball_C" (`SceneComponent.K2_GetComponentToWorld` (`/Game/MainCharacterBP/Blueprints/MainCharacterBP.SpellDirection` (`self.As Main Character BP`))) "Undefined" "OverrideRootScale" null 1.0 20.0 null))