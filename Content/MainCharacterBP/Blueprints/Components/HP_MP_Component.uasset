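; Actor component that tracks health and mana for a character, with damage and death-flag handling.
; ConsumeMP deducts mana when enough is available, then starts regeneration behind a DoOnce gate that prevents overlapping runs.
; A delay-looping macro restores mana per tick up to the maximum, updating the HP/MP bar widget fetched from the player's main widget.
; A generic delayed while-loop macro is also defined but unused here.
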(event `self.ReceiveBeginPlay`
  (`KismetSystemLibrary.Delay` 0.2)
  (set `self.HP MP Bar WB` (`/Game/Terrain/UI/Widgets/MainWB.HP_MP_Bar_WB` (`/Game/MainCharacterBP/Blueprints/MainCharacterBP.MainWB` (cast `/Game/MainCharacterBP/Blueprints/MainCharacterBP` (`GameplayStatics.GetPlayerCharacter` 0) :!pure true)))))

(event `Consume MP`
  (params (`MP Cost` :type "Float (double-precision)"))
  (`self.MP Consumption Input` `MP Cost`)
  ;[1 1 1] Prevent multiple mana regeneration
  (`/Engine/EditorBlueprintResources/StandardMacros.DoOnce` false :!label _label
    (:`Completed`
      (`self.MP Regeneration`
        (:`Completed`
          (goto _label :!via `Reset`))))))

(fn `Damage Input`
  (params (Damage :type "Float (double-precision)"))
  (locals (`Local Damage` :type "Float (double-precision)"))
  (set `local.Local Damage` Damage)
  (if (< (`self.Current HP`) (`local.Local Damage`))
    (set `self.Current HP` 0.0)
    (set `self.IsDead` true)
    (else
      (set `self.Current HP` (- (`self.Current HP`) (`local.Local Damage`))))))

(fn `MP Consumption Input`
  (params (`MP To Consume` :type "Float (double-precision)"))
  (locals (`Local MP To Consume` :type "Float (double-precision)"))
  (set `local.Local MP To Consume` `MP To Consume`)
  (if (not (> (`local.Local MP To Consume`) (`self.Current MP`)))
    ;[1 1 1] If there is enough mana for spell, it consumes
    (set `self.Current MP` (- (`self.Current MP`) (`local.Local MP To Consume`)))))

(fn `Set HP and MP`
  (params (`Current HP` :type "Float (double-precision)") (`Max HP` :type "Float (double-precision)") (`Current MP` :type "Float (double-precision)") (`Max MP` :type "Float (double-precision)"))
  (set `self.Current HP` `Current HP`)
  (set `self.Max HP` `Max HP`)
  (set `self.Current MP` `Current MP`)
  (set `self.Max MP` `Max MP`))